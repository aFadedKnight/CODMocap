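; BP_Lightning simulates recurring lightning flashes by driving the intensity of a directional light.
; A timer fires E_Flash after a random delay, which gives the light a random yaw and plays the lightning timeline at a random rate.
; The timeline's curve is remapped to light intensity, and its completion schedules the next flash, so the cycle repeats indefinitely from BeginPlay.
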(event Custom|E_Flash
  (bind _directionallight (Variables|Default|GetDirectionalLight))
  (bind _returnvalue (Transformation|GetWorldRotation _directionallight))
  (Transformation|SetWorldRotation _directionallight (Math|Rotator|MakeRotator (.roll _returnvalue) (.pitch _returnvalue) (Math|Random|RandomFloatinRange 0.0 3.6e+02)) false false)
  (Components|Timeline|SetPlayRate (Variables|Default|GetT_Lightning) (Math|Random|RandomFloatinRange 0.5 1.0))
  (bind _0_1 (Timeline|T_Lightning PlayFromStart)
    (:Update
      (Rendering|Components|Light|SetIntensity (Variables|Default|GetDirectionalLight) (Math|Float|MapRangeClamped _0_1 0.0 1.0 0.0 8.0)))
    (:Finished
      (Utilities|Time|SetTimerbyFunctionName 0 "E_Flash" (Math|Random|RandomFloatinRange 3.0 1e+01)))))

(event EventBeginPlay
  (Utilities|Time|SetTimerbyFunctionName 0 "E_Flash" (Math|Random|RandomFloatinRange 3.0 1e+01)))

(fn ConstructionScript)