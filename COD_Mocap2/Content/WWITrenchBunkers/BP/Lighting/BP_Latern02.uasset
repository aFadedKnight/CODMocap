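; Lantern lighting Blueprint that makes its point light flicker at irregular intervals during play.
; On BeginPlay, a randomly delayed timer calls E_Flicker, which randomizes the timeline's play rate and plays it from the start.
; The timeline's track is remapped to point light intensity on each update, and its completion re-arms the timer with a new random delay, so the flicker repeats indefinitely without Tick.
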(event Custom|E_Flicker
  (Components|Timeline|SetPlayRate (Variables|Default|GetT_Flicker) (Math|Random|RandomFloatinRange 0.5 1.0))
  (bind _0_1 (Timeline|T_Flicker PlayFromStart)
    (:Update
      (Rendering|Components|Light|SetIntensity (Variables|Default|GetPointLight) (Math|Float|MapRangeClamped _0_1 0.0 1.0 0.0 3e+03)))
    (:Finished
      (Utilities|Time|SetTimerbyFunctionName 0 "E_Flicker" (Math|Random|RandomFloatinRange 1.0 5.0)))))

(event EventBeginPlay
  (Utilities|Time|SetTimerbyFunctionName 0 "E_Flicker" (Math|Random|RandomFloatinRange 1.0 5.0)))

(event Collision|EventActorBeginOverlap
  (params (OtherActor :type Actor%20Object%20Reference)))

(event EventTick
  (params (DeltaSeconds :type Float%20%28single-precision%29)))

(fn ConstructionScript)